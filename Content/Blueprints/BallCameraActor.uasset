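; BallCameraActor is a shared camera that tracks the ball (first Ballsack actor) for Footballer players.
; On BeginPlay it becomes the view target of Footballers' player controllers.
; Each Tick it follows the ball along clamped X, keeping its Y and Z, and pitches toward it within a narrow downward range at fixed yaw.
; A successful move also re-runs the view-target assignment, repeating the actor searches during play.
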(event `self.ReceiveBeginPlay`
  (bind _outactors (`GameplayStatics.GetAllActorsOfClass` "/Script/OSF.Footballer" :!label _label))
  (for _array_element _outactors
    (bind _asplayer_controller (cast `PlayerController` (`Pawn.GetController` _array_element)))
    (`PlayerController.SetViewTargetWithBlend` _asplayer_controller self 0.0 "VTBlend_Linear" 0.0 false)))

(event `self.ReceiveActorBeginOverlap`
  (params (OtherActor :type "Actor Object Reference")))

(event `self.ReceiveTick`
  (params (DeltaSeconds :type "Float (single-precision)"))
  (bind _outactors (`GameplayStatics.GetAllActorsOfClass` "/Script/OSF.Ballsack"))
  (bind _returnvalue (`self.K2_GetActorLocation` (`KismetArrayLibrary.Array_Get` _outactors)))
  (bind _returnvalue_2 (`KismetMathLibrary.MakeVector` (`KismetMathLibrary.FClamp` (.x _returnvalue) -3000.0 3000.0) (.y (`self.K2_GetActorLocation` self)) (.z (`self.K2_GetActorLocation` self))))
  (bind (_sweephitresult _returnvalue_3) (`self.K2_SetActorLocation` _returnvalue_2))
  (`self.SetActorRotation` (`KismetMathLibrary.MakeRotator` 0.0 (`KismetMathLibrary.ClampAngle` (.pitch (`KismetMathLibrary.FindLookAtRotation` _returnvalue_2 _returnvalue)) -55.0 -45.0) -90.0))
  (if _returnvalue_3
    (goto _label)))

(fn `UserConstructionScript`)