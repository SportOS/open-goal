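; Behavior tree service that decides whether an AI-controlled footballer should press the ball.
; Each tick it asks the pawn's team for the footballer closest to the ball and sets ShouldBePressing true only if that is this pawn.
; It also writes the ball's current location to the TargetLocation blackboard key.
; A distance-to-ball threshold check is present but unused.
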(event `self.ReceiveTick`
  (params (OwnerActor :type "Actor Object Reference") (DeltaSeconds :type "Float (single-precision)"))
  (bind _returnvalue (`AIBlueprintHelperLibrary.GetAIController` OwnerActor))
  (bind _asbpfootballer (cast `/Game/Blueprints/BPFootballer` (`Controller.K2_GetPawn` _returnvalue)))
  (bind _ball (`Footballer.Ball` _asbpfootballer))
  (bind _returnvalue_2 (`FootballTeam.GetClosestFootballerToBall` (`Footballer.Team` _asbpfootballer) _ball))
  (`BTFunctionLibrary.SetBlackboardValueAsBool` (`self.ShouldBePressing`) (== _returnvalue_2 _asbpfootballer))
  (`BTFunctionLibrary.SetBlackboardValueAsVector` (`self.TargetLocation`) (`Actor.K2_GetActorLocation` _ball)))